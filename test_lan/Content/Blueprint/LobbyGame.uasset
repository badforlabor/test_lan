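; LobbyGame is the lobby Blueprint that shows the lobby menu and handles hosting or joining LAN multiplayer games.
; On BeginPlay it adds the LobbyPage widget to the viewport and shows the mouse cursor.
; CreateGame creates a LAN session, then opens ThirdPersonExampleMap as a listen server.
; JoinGame searches for LAN sessions and joins the first one found, with debug prints only on success.
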(event Custom|CreateGame
  (|Session (Game|GetPlayerController 0) 8 true
    (:OnSuccess
      (Development|PrintString "create game succ")
      (Game|OpenLevel(byName) "/Game/ThirdPersonBP/Maps/ThirdPersonExampleMap" true "listen"))))

(event Custom|JoinGame
  (bind _returnvalue (Game|GetPlayerController 0))
  (bind _results (|FindSessions _returnvalue 10 true)
    (:OnSuccess
      (if (> (Utilities|Array|Length _results) 0)
        (Development|PrintString "find session suc")
        (|JoinSession _returnvalue (Utilities|Array|Get(acopy) _results))))))

(event EventBeginPlay
  (bind _returnvalue (UserInterface|CreateWidget "/Game/UI/LobbyPage.LobbyPage_C"))
  (UserInterface|Viewport|AddtoViewport _returnvalue 0)
  (Variables|/Script/Engine.PlayerController|SetbShowMouseCursor (Game|GetPlayerController 0) true))

(event EventTick
  (params (DeltaSeconds :type Float%20%28single-precision%29)))

(fn ConstructionScript)